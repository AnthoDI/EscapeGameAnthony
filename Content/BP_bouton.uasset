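; BP_bouton is a button trigger that records in the first-person game mode that the player has touched it.
; On BeginPlay, GetBluePrints caches the player character and the game mode.
; When the player overlaps component R, the Button1 boolean selects whether the game mode's Button1 or Button2 flag is set to true, with a debug print.
; Nothing here resets either flag.
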(event OnComponentBeginOverlap(r)
  (params (OverlappedComponent :type Primitive%20Component%20Object%20Reference) (OtherActor :type Actor%20Object%20Reference) (OtherComp :type Primitive%20Component%20Object%20Reference) (OtherBodyIndex :type Integer) (bFromSweep :type Boolean) (SweepResult :type Hit%20Result%20Structure%20%28by%20ref%29))
  (if (== OtherActor (Variables|Default|GetAs%20BP%20First%20Person%20Character))
    (if (Variables|Default|Getbutton1%20?)
      (Variables|/Game/FirstPerson/Blueprints/BP_FirstPersonGameMode.BP_FirstPersonGameMode_C|SetButton1 (Variables|Default|GetAs%20BP%20First%20Person%20Game%20Mode) true)
      (Development|PrintString "1 true")
      (else
        (Variables|/Game/FirstPerson/Blueprints/BP_FirstPersonGameMode.BP_FirstPersonGameMode_C|SetButton2 (Variables|Default|GetAs%20BP%20First%20Person%20Game%20Mode) true)
        (Development|PrintString "2 true")))))

(event EventBeginPlay
  (CallFunction|GetBluePrints))

(fn ConstructionScript)

(fn GetBluePrints
  (Utilities|FlowControl|Sequence
    (:then_0
      (bind _asfirst_person_character (Utilities|Casting|CastToFirstPersonCharacter (Game|GetPlayerCharacter 0)))
      (Variables|Default|SetAs%20BP%20First%20Person%20Character _asfirst_person_character))
    (:then_1
      (bind _asbp_first_person_game_mode (Utilities|Casting|CastToBP_FirstPersonGameMode (Game|GetGameMode)))
      (Variables|Default|SetAs%20BP%20First%20Person%20Game%20Mode _asbp_first_person_game_mode))))